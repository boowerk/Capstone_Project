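; Biome manager actor that feeds a biome's item groups into a PCG graph instance.
; On BeginPlay it looks up a hardcoded "Ruins" entry in BiomeMap, where a comment indicates the name is meant to come from an LLM.
; For each CategoryKeys entry found in that biome's ItemGroups, it sets the graph's object parameter of the same name to that group's value.
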(event EventBeginPlay
  (bind _biomemap (Variables|Default|GetBiomeMap))
  (bind (_value _returnvalue) (Utilities|Map|Find _biomemap "Ruins"))
  (if _returnvalue
    (Variables|Default|SetFoundBiomeGroups (Variables|/Script/Project_Eden.PDA_Biome|GetItemGroups _value))
    (for _array_element (Variables|Default|GetCategoryKeys)
      (if (.ReturnValue (Utilities|Map|Find (Variables|Default|GetFoundBiomeGroups) _array_element))
        (Audio|Parameter|SetObjectParameter (Variables|/Script/PCG.PCGComponent|GetGraphInstance (Variables|Default|GetPCG)) _array_element (Utilities|ResolveSoftReference (.Value (Utilities|Map|Find (Variables|Default|GetFoundBiomeGroups) _array_element))))))))

(event Collision|EventActorBeginOverlap
  (params (OtherActor :type Actor%20Object%20Reference)))

(event EventTick
  (params (DeltaSeconds :type Float%20%28single-precision%29)))

(fn ConstructionScript)